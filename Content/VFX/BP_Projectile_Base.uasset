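; BP_Projectile_Base is a base projectile that flies via a ProjectileMovement component and explodes on impact.
; The construction script applies the Speed variable to both initial and max speed, and Gravity to the gravity scale.
; When its Box component hits, it fires the projectile-impact dispatcher with the hit actor and result, spawns an effect system and explosion sound at the hit location, then destroys itself.
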(event OnComponentHit(Box)
  (params (HitComponent :type Primitive%20Component%20Object%20Reference) (OtherActor :type Actor%20Object%20Reference) (OtherComp :type Primitive%20Component%20Object%20Reference) (NormalImpulse :type Vector :default "0, 0, 0") (Hit :type Hit%20Result%20Structure%20%28by%20ref%29))
  (bind _location (Collision|BreakHitResult Hit))
  (Default|CallOnprojectileimpact OtherActor Hit)
  (Niagara|SpawnSystematLocation (Variables|effects|GetSystem%20Template) _location)
  (Audio|PlaySoundatLocation "/Game/StarterContent/Audio/Explosion01.Explosion01" _location "0, 0, 0" 1.0 1.0 0.0 0 0 0 0)
  (Actor|DestroyActor))

(fn ConstructionScript
  (bind _projectilemovement (Variables|Default|GetProjectileMovement))
  (Variables|/Script/Engine.ProjectileMovementComponent|SetInitialSpeed _projectilemovement (Variables|projectileSettings|Getspeed))
  (Variables|/Script/Engine.ProjectileMovementComponent|SetMaxSpeed _projectilemovement (Variables|projectileSettings|Getspeed))
  (Variables|/Script/Engine.ProjectileMovementComponent|SetProjectileGravityScale _projectilemovement (Variables|projectileSettings|Getgravity)))